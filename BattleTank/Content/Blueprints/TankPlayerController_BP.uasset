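; Player controller Blueprint for the tank game that sets up the player's UI.
; The SetPlayerUI event casts the controlled pawn to Tank_BP, adds a PlayerUI widget to the viewport and gives it that tank reference.
; Disconnected leftover test nodes fire a projectile from the barrel socket toward the sight-ray hit point using Suggest Projectile Velocity, but never run.
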(event EventTick
  (params (DeltaSeconds :type Float%20%28single-precision%29)))

(event EventSetPlayerUI
  (bind _astank_bp (Utilities|Casting|CastToTank_BP (Pawn|GetControlledPawn)))
  (bind _returnvalue (UserInterface|CreateWidget "/Game/UI/PlayerUI.PlayerUI_C"))
  (UserInterface|Viewport|AddtoViewport _returnvalue 0)
  (Variables|/Game/UI/PlayerUI.PlayerUI_C|SetPlayerTank _returnvalue _astank_bp))

(fn ConstructionScript)